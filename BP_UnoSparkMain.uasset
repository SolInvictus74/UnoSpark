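; BP_UnoSparkMain is a function library-style Blueprint for modding Korat character and action data assets at runtime.
; Most functions use LoadCastFindCharData to blocking-load a character's record, then write bullets, combatives, combinations, MLS or stats, while AddAction registers new actions.
; SwapMoveset copies another character's combatives and MLS, then restores signature action groups from the original.
; Init is empty; author notes mark StorySettingParameter as broken and SwapMoveset as risky.
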(event `/SZModLib/Blueprints/Interfaces/BPI_ModObjects.Init`)

(fn `Add Action`
  (params (ActKey :type Name) (`Data Asset` :type "SSActionDataAsset Object Reference") (`Sort Id` :type Integer))
  (bind _returnvalue (`KismetSystemLibrary.LoadAsset_Blocking` "/Game/SS/Blueprints/ActionData.ActionData"))
  (bind _askorat_action_data_asset (cast `KoratActionDataAsset` _returnvalue))
  (`BlueprintMapLibrary.Map_Add` (`KoratActionDataAsset.Records` _askorat_action_data_asset) ActKey (make `KoratActionDataAssetRecord` `Data Asset` ActKey `Sort Id`)))

(fn `BulletSetting`
  (params (CharacterID :type "Name (by ref)") (Key :type Name) (Parameter :type "SSBulletParamDataAsset Object Reference") (`Bullet Actor BP` :type "SSBulletActor Soft Class Reference") (`Effect Key` :type Name))
  ;[1 1 1] I recommend having an open Bullet Setting before your eyes to fully understand what this function does and what it allows you to change
  (bind _character_data_asset_record (`self.LoadCastFind(CharData)` CharacterID))
  (bind ((`CommonAssets` _commonassets)) (break `KoratCharacterDataAssetRecord` _character_data_asset_record))
  (setmembers `KoratCharacterDataCommonAssets` :`StructRef` _commonassets)
  (`BlueprintMapLibrary.Map_Add` (`SSBulletSettingDataAsset.RecordsByDataList` (`.BulletSettingData` (break `KoratCharacterDataCommonAssets` _commonassets))) (make `KoratActionDataList` Key) (make `SSBulletDataAssetRecordParam` (struct) null null (`|MakeMap` (make `KoratBulletKeyDataList` "None") (make `SSBulletDataAssetRecordParamAdditional` (make `KoratBulletEffectDataList` `Effect Key`) Parameter `Bullet Actor BP`) :!type "KoratBulletKeyDataList Structure" :!valuetype "SSBulletDataAssetRecordParamAdditional Structure"))))

(fn `BulletVisual`
  (params (CharacterID :type "Name (by ref)") (`ULT/SPM1/SPM2` :type Name) (`Bullet Level Sequence In` :type "LevelSequence Soft Object Reference"))
  (locals (JapaneseKey :type Name :default "None"))
  (bind _japanesekey (`local.JapaneseKey`))
  (if (== `ULT/SPM1/SPM2` "ULT")
    (set `local.JapaneseKey` "アルティメットブラスト")
    (bind _character_data_asset_record (`self.LoadCastFind(CharData)` CharacterID :!label _label))
    (bind ((`CommonAssets` _commonassets)) (break `KoratCharacterDataAssetRecord` _character_data_asset_record))
    (setmembers `KoratCharacterDataCommonAssets` :`StructRef` _commonassets)
    (`BlueprintMapLibrary.Map_Add` (`SSBulletVisualDataAsset.RecordsByDataList` (`.BulletVisualData` (break `KoratCharacterDataCommonAssets` _commonassets))) (make `KoratBulletEffectDataList` _japanesekey) (make `SSBulletDataAssetRecordEffect` (make `KoratBulletEffectDataList` _japanesekey) `Bullet Level Sequence In`))
    (elif (== `ULT/SPM1/SPM2` "SPM1")
      (set `local.JapaneseKey` "必殺技１")
      (goto _label)
      (elif (== `ULT/SPM1/SPM2` "SPM2")
        (set `local.JapaneseKey` "必殺技２")
        (goto _label)))))

(fn `Combatives`
  (params (CharacterID :type "Name (by ref)") (ActionKey :type "Name (by ref)") (Parameter :type "SSCombativesDataAsset Object Reference") (`Sub Parameter` :type "SSCombativesSubDataAsset Object Reference") (Visual :type "SSCombativesVisualDataAsset Object Reference"))
  (bind _character_data_asset_record (`self.LoadCastFind(CharData)` CharacterID))
  (`BlueprintMapLibrary.Map_Add` (`SSCharacterCombativesDataAsset.PtrRecords2` (`.CombativesData` (break `KoratCharacterDataCommonAssets` (`.CommonAssets` (break `KoratCharacterDataAssetRecord` _character_data_asset_record))))) ActionKey (make `SSCharacterCombativesDataAssetRecordParam` null null null (`|MakeMap` (make `KoratCombativesKeyDataList` "None") (make `SSCharacterCombativesDataAssetRecordParamAdditional` _ Parameter `Sub Parameter` Visual) :!type "KoratCombativesKeyDataList Structure" :!valuetype "SSCharacterCombativesDataAssetRecordParamAdditional Structure"))))

(fn `Combination`
  (params (CharacterID :type "Name (by ref)") (`Action Key` :type Name) (`Action Opponent Key` :type Name) (`Data Asset` :type "KoratCombinationDataAsset Object Reference"))
  (bind _character_data_asset_record (`self.LoadCastFind(CharData)` CharacterID))
  (`BlueprintMapLibrary.Map_Add` (`KoratCharacterCombinationDataAsset.Records` (`.CharacterCombination` (break `KoratCharacterDataAssetRecord` _character_data_asset_record))) (make `KoratActionDataList` `Action Key`) (make `KoratCharacterCombinationDataAssetRecord` (make `KoratActionDataList` `Action Opponent Key`) _ `Data Asset`)))

(fn `LoadCastFind(CharData)`
  (params (CharacterID :type Name))
  (returns (`Character Data Asset Record` :type "KoratCharacterDataAssetRecord Structure"))
  (bind _returnvalue (`KismetSystemLibrary.LoadAsset_Blocking` "/Game/SS/Blueprints/CharacterData.CharacterData"))
  (bind _askorat_character_data_asset (cast `KoratCharacterDataAsset` _returnvalue))
  (bind (_value _returnvalue_2) (`BlueprintMapLibrary.Map_Find` (`KoratCharacterDataAsset.PtrRecords` _askorat_character_data_asset) CharacterID))
  (if _returnvalue_2
    (return (`SSCharacterDataAsset.CharacterDataAssetRecord` _value))))

(fn `NumericData`
  (params (CharacterID :type "Name (by ref)") (Life :type "Float (single-precision)") (`Blast Stock` :type Integer) (`Initial Blast Stock` :type Integer) (`Aura Type` :type "EKoratBattleAuraType Enum" :default "None") (`Damage Rate` :type "Float (single-precision)"))
  (locals (NewLocalVar :type Boolean))
  (bind _character_data_asset_record (`self.LoadCastFind(CharData)` CharacterID))
  (bind ((`NumericData` _numericdata)) (break `KoratCharacterDataCommonAssets` (`.CommonAssets` (break `KoratCharacterDataAssetRecord` _character_data_asset_record))))
  (set `SSNumericDataAsset.Life` Life _numericdata)
  (set `SSNumericDataAsset.BlastStock` `Blast Stock` _numericdata)
  (set `SSNumericDataAsset.AuraType` `Aura Type` _numericdata)
  (set `SSNumericDataAsset.InitialBlastStock` `Initial Blast Stock` _numericdata)
  (set `SSNumericDataAsset.DamageRate` `Damage Rate` _numericdata))

(fn `PersonalizeAction`
  (params (CharacterID :type Name) (ActionKey :type Name) (MLSData :type "KoratMLSDataAsset Object Reference"))
  (bind _character_data_asset_record (`self.LoadCastFind(CharData)` CharacterID))
  (setmembers `KoratCharacterDataAssetRecord` :`StructRef` _character_data_asset_record)
  (`BlueprintMapLibrary.Map_Add` (`KoratCharacterMLSDataAsset.PtrRecordsByDataList` (`.CharacterMLS` (break `KoratCharacterDataAssetRecord` _character_data_asset_record))) (make `KoratActionDataList` ActionKey) MLSData))

(fn `StorySettingParameter`
  (params (CharacterID :type "Name (by ref)") (Gender :type "EKoratCharacterGenderType Enum" :default "None") (`First Form` :type Boolean) (`Ruby Sort Id` :type Integer) (`Appeared Sort Id` :type Integer) (`Sort Id` :type Integer) (`Maintain SamePersons as Zerospark?` :type Boolean))
  (bind _character_data_asset_record (`self.LoadCastFind(CharData)` CharacterID))
  (bind ((`StorySettingParameter` _storysettingparameter)) (break `KoratCharacterDataAssetRecord` _character_data_asset_record))
  (bind ((`DestroyedPower` _destroyedpower) (`CharacterType` _charactertype) (`SeriesTitle` _seriestitle) (`SeriesTitleList` _seriestitlelist) (`Species` _species) (`CharacterAttributeTagData` _characterattributetagdata) (`SamePersons` _samepersons) (`Group` _group)) (break `KoratCharacterDataStorySettingParameter` _storysettingparameter))
  (setmembers `KoratCharacterDataStorySettingParameter` :`StructRef` _storysettingparameter :`SortId` `Sort Id` :`AppearedSortId` `Appeared Sort Id` :`RubySortId` `Ruby Sort Id` :`DestroyedPower` _destroyedpower :`CharacterType` _charactertype :`SeriesTitle` _seriestitle :`SeriesTitleList` _seriestitlelist :`Species` _species :`CharacterAttributeTagData` _characterattributetagdata :`Gender` Gender :`SamePersons` _samepersons :`Group` _group :`bFirstForm` `First Form`))

(fn `Swap Moveset(A Restore MLS)`
  (params (Array :type "Array of Name") (OriginalMLS :type "Map of KoratActionDataList Structure to KoratMLSDataAsset Object Reference (by ref)") (CharacterID :type Name))
  (`self.FunctionRemoveCharacterAction` CharacterID Array)
  (bind _character_data_asset_record (`self.LoadCastFind(CharData)` CharacterID))
  (for _array_element Array
    (bind _koratactiondatalist (make `KoratActionDataList` _array_element))
    (bind (_value _returnvalue) (`BlueprintMapLibrary.Map_Find` OriginalMLS _koratactiondatalist))
    (if _returnvalue
      (`BlueprintMapLibrary.Map_Add` (`KoratCharacterMLSDataAsset.PtrRecordsByDataList` (`.CharacterMLS` (break `KoratCharacterDataAssetRecord` _character_data_asset_record))) _koratactiondatalist _value))))

(fn `SwapMoveset`
  (params (`CharacterID (CopyMovesetFrom)` :type "Name (by ref)") (CharacterID :type Name) (`Keep Jump Ki Blasts?` :type Boolean))
  (locals (OriginalRecordsCombatives :type "Map of KoratActionDataList Structure to SSCharacterCombativesDataAssetRecordParam Structure") (OriginalRecordMLS :type "Map of KoratActionDataList Structure to KoratMLSDataAsset Object Reference") (ChangedRecordsCombatives :type "Map of KoratActionDataList Structure to SSCharacterCombativesDataAssetRecordParam Structure") (ChangedRecordsMLS :type "Map of KoratActionDataList Structure to KoratMLSDataAsset Object Reference") (OriginalCharDataRecords :type "KoratCharacterDataAssetRecord Structure"))
  (bind _originalrecordmls (`local.OriginalRecordMLS`))
  (bind _jumpkiprojectile (`self.JumpKiProjectile`))
  (bind _originalrecordscombatives (`local.OriginalRecordsCombatives`))
  (bind _character_data_asset_record (`self.LoadCastFind(CharData)` CharacterID))
  (set `self.OriginalCharacterDataAssetRecord` _character_data_asset_record)
  (bind _character_data_asset_record_2 (`self.LoadCastFind(CharData)` `CharacterID (CopyMovesetFrom)`))
  (bind _recordsbydatalist (`SSCharacterCombativesDataAsset.RecordsByDataList` (`.CombativesData` (break `KoratCharacterDataCommonAssets` (`.CommonAssets` (break `KoratCharacterDataAssetRecord` _character_data_asset_record))))))
  ;[1 1 1] Combatives
  (set `local.OriginalRecordsCombatives` _recordsbydatalist)
  (bind _recordsbydatalist_2 (`SSCharacterCombativesDataAsset.RecordsByDataList` (`.CombativesData` (break `KoratCharacterDataCommonAssets` (`.CommonAssets` (break `KoratCharacterDataAssetRecord` _character_data_asset_record_2))))))
  (set `local.ChangedRecordsCombatives` _recordsbydatalist_2)
  (bind _keys (`BlueprintMapLibrary.Map_Keys` _recordsbydatalist_2))
  (for _array_element _keys
    (bind (_value _returnvalue) (`BlueprintMapLibrary.Map_Find` _recordsbydatalist_2 _array_element))
    (if _returnvalue
      (`BlueprintMapLibrary.Map_Add` _recordsbydatalist _array_element _value)))
  (bind _ptrrecordsbydatalist (`KoratCharacterMLSDataAsset.PtrRecordsByDataList` (`.CharacterMLS` (break `KoratCharacterDataAssetRecord` _character_data_asset_record))))
  ;[1 1 1] MLS
  (set `local.OriginalRecordMLS` _ptrrecordsbydatalist)
  (set `local.ChangedRecordsMLS` _ptrrecordsbydatalist)
  (bind _ptrrecordsbydatalist_2 (`KoratCharacterMLSDataAsset.PtrRecordsByDataList` (`.CharacterMLS` (break `KoratCharacterDataAssetRecord` _character_data_asset_record_2))))
  (bind _keys_2 (`BlueprintMapLibrary.Map_Keys` _ptrrecordsbydatalist_2))
  (for _array_element_2 _keys_2
    (bind (_value_2 _returnvalue_2) (`BlueprintMapLibrary.Map_Find` _ptrrecordsbydatalist_2 _array_element_2))
    (if _returnvalue_2
      (`BlueprintMapLibrary.Map_Add` _ptrrecordsbydatalist _array_element_2 _value_2)))
  ;[1 1 1] RestoreCombination
  (`self.SwapMoveset(ARestoreCombatives)` (`self.Intro_Action_Files`) CharacterID _originalrecordscombatives)
  (`self.SwapMoveset(ARestoreCombatives)` (`self.Throw_Action_Files`) CharacterID _originalrecordscombatives)
  (`self.SwapMoveset(ARestoreCombatives)` (`self.Charge_Action_Files`) CharacterID _originalrecordscombatives)
  (`self.SwapMoveset(ARestoreCombatives)` (`self.Skill2_Action_Files`) CharacterID _originalrecordscombatives)
  (`self.SwapMoveset(ARestoreCombatives)` (`self.Skill1_Action_Files`) CharacterID _originalrecordscombatives)
  (`self.SwapMoveset(ARestoreCombatives)` (`self.Blast1_Action_Files`) CharacterID _originalrecordscombatives)
  (`self.SwapMoveset(ARestoreCombatives)` (`self.Blast2_Action_Files`) CharacterID _originalrecordscombatives)
  (`self.SwapMoveset(ARestoreCombatives)` (`self.Ultimate_Action_Files`) CharacterID _originalrecordscombatives)
  ;[1 1 1] RestoreMLS
  (`self.Swap Moveset(A Restore MLS)` (`self.Intro_Action_Files`) _originalrecordmls CharacterID)
  (`self.Swap Moveset(A Restore MLS)` (`self.Throw_Action_Files`) _originalrecordmls CharacterID)
  (`self.Swap Moveset(A Restore MLS)` (`self.Charge_Action_Files`) _originalrecordmls CharacterID)
  (`self.Swap Moveset(A Restore MLS)` (`self.Blast1_Action_Files`) _originalrecordmls CharacterID)
  (`self.Swap Moveset(A Restore MLS)` (`self.Blast2_Action_Files`) _originalrecordmls CharacterID)
  (`self.Swap Moveset(A Restore MLS)` (`self.Skill1_Action_Files`) _originalrecordmls CharacterID)
  (`self.Swap Moveset(A Restore MLS)` (`self.Skill2_Action_Files`) _originalrecordmls CharacterID)
  (`self.Swap Moveset(A Restore MLS)` (`self.Ultimate_Action_Files`) _originalrecordmls CharacterID)
  (`self.Swap Moveset(A Restore MLS)` (`self.Transformation_Action_Files`) _originalrecordmls CharacterID)
  (`self.Swap Moveset(A Restore MLS)` (`self.Win_Action_Files`) _originalrecordmls CharacterID)
  (`self.Swap Moveset(A Restore MLS)` (`self.Power_Up_1_Action_Files`) _originalrecordmls CharacterID)
  (`self.Swap Moveset(A Restore MLS)` (`self.Power_Up_2_Action_Files`) _originalrecordmls CharacterID)
  (`self.Swap Moveset(A Restore MLS)` (`self.Power_Up_3_Action_Files`) _originalrecordmls CharacterID)
  (`self.Swap Moveset(A Restore MLS)` (`self.Power_Down_Action_Files`) _originalrecordmls CharacterID)
  (`self.Swap Moveset(A Restore MLS)` (`self.Potara_Action_Files`) _originalrecordmls CharacterID)
  (`self.Swap Moveset(A Restore MLS)` (`self.Fusion_Action_Files`) _originalrecordmls CharacterID)
  (`self.Swap Moveset(A Restore MLS)` (`self.Power_Up_Result`) _originalrecordmls CharacterID)
  (if `Keep Jump Ki Blasts?`
    (`self.SwapMoveset(KRestoreMLS)` (`local.OriginalRecordMLS`) _jumpkiprojectile CharacterID)
    (`self.SwapMoveset(KRestoreCombatives)` (`local.OriginalRecordsCombatives`) _jumpkiprojectile CharacterID))
  (return))

(fn `SwapMoveset(ARestoreCombatives)`
  (params (Array :type "Array of Name") (CharacterID :type Name) (OriginalCombatives :type "Map of KoratActionDataList Structure to SSCharacterCombativesDataAssetRecordParam Structure (by ref)"))
  (`self.FunctionRemoveCharacterAction` CharacterID Array)
  (bind _character_data_asset_record (`self.LoadCastFind(CharData)` CharacterID))
  (for _array_element Array
    (bind _koratactiondatalist (make `KoratActionDataList` _array_element))
    (bind (_value _returnvalue) (`BlueprintMapLibrary.Map_Find` OriginalCombatives _koratactiondatalist))
    (if _returnvalue
      (`BlueprintMapLibrary.Map_Add` (`SSCharacterCombativesDataAsset.RecordsByDataList` (`.CombativesData` (break `KoratCharacterDataCommonAssets` (`.CommonAssets` (break `KoratCharacterDataAssetRecord` _character_data_asset_record))))) _koratactiondatalist _value))))

(fn `SwapMoveset(KRestoreCombatives)`
  (params (OriginalCombatives :type "Map of KoratActionDataList Structure to SSCharacterCombativesDataAssetRecordParam Structure (by ref)") (Key :type Name) (CharacterID :type Name))
  (bind (_value _returnvalue) (`BlueprintMapLibrary.Map_Find` OriginalCombatives))
  (bind _koratactiondatalist (make `KoratActionDataList` Key))
  (bind _character_data_asset_record (`self.LoadCastFind(CharData)` CharacterID))
  (bind _recordsbydatalist (`SSCharacterCombativesDataAsset.RecordsByDataList` (`.CombativesData` (break `KoratCharacterDataCommonAssets` (`.CommonAssets` (break `KoratCharacterDataAssetRecord` _character_data_asset_record))))))
  (`BlueprintMapLibrary.Map_Remove` _recordsbydatalist _koratactiondatalist)
  (if _returnvalue
    (`BlueprintMapLibrary.Map_Add` _recordsbydatalist _koratactiondatalist _value))
  (return))

(fn `SwapMoveset(KRestoreMLS)`
  (params (OriginalMLS :type "Map of KoratActionDataList Structure to KoratMLSDataAsset Object Reference (by ref)") (Key :type Name) (CharacterID :type Name))
  (bind _koratactiondatalist (make `KoratActionDataList` Key))
  (bind (_value _returnvalue) (`BlueprintMapLibrary.Map_Find` OriginalMLS _koratactiondatalist))
  (bind _character_data_asset_record (`self.LoadCastFind(CharData)` CharacterID))
  (bind _ptrrecordsbydatalist (`KoratCharacterMLSDataAsset.PtrRecordsByDataList` (`.CharacterMLS` (break `KoratCharacterDataAssetRecord` _character_data_asset_record))))
  (`BlueprintMapLibrary.Map_Remove` _ptrrecordsbydatalist _koratactiondatalist)
  (if _returnvalue
    (`BlueprintMapLibrary.Map_Add` _ptrrecordsbydatalist _koratactiondatalist _value)
    (return)))